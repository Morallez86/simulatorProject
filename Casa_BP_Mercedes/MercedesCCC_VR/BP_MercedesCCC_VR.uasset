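; Drivable Mercedes CCC vehicle for VR that sends motion feedback to a YawController.
; At start, if an HMD is enabled, it offsets the camera root and sets eye-level tracking.
; Throttle, brake and steering axes drive VehicleMovement, then each updates the YawController with a computed rotation.
; GetRotationFromAxis smooths roll from turn and pitch from thrust minus brake, both scaled by clamped forward speed.
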(event EventBeginPlay
  (Utilities|FlowControl|Delay 0.05)
  (if (Class|HeadMountedDisplayFunctionLibrary|IsHeadMountedDisplayEnabled)
    (Transformation|AddLocalOffset (Variables|Default|GetCameraRoot) (+ (Variables|/Script/Engine.SceneComponent|GetRelativeLocation (Variables|Default|GetVRCamera)) "10.000000, 0,6.000000") false false)
    (Class|HeadMountedDisplayFunctionLibrary|SetTrackingOrigin "Eye")))

(event Collision|EventActorBeginOverlap
  (params (OtherActor :type Actor%20Object%20Reference)))

(event Input|AxisEvents|InputAxisMoveRight
  (params (AxisValue :type Float%20%28single-precision%29))
  (Class|WheeledVehicleMovementComponent|SetSteeringInput (Variables|Default|GetVehicleMovement) AxisValue)
  (bind _newparam3 (CallFunction|GetRotationfromAxis AxisValue (stale Input|AxisEvents|InputAxisMoveFoward AxisValue) (stale Input|AxisEvents|InputAxisBrake AxisValue)))
  (Class|YawController|UpdateMotionValues (Variables|Default|GetYawController) _newparam3))

(event Input|AxisEvents|InputAxisMoveFoward
  (params (AxisValue :type Float%20%28single-precision%29))
  (Class|WheeledVehicleMovementComponent|SetThrottleInput (Variables|Default|GetVehicleMovement) AxisValue)
  (bind _newparam3 (CallFunction|GetRotationfromAxis (stale Input|AxisEvents|InputAxisMoveRight AxisValue) AxisValue (stale Input|AxisEvents|InputAxisBrake AxisValue)))
  (Class|YawController|UpdateMotionValues (Variables|Default|GetYawController) _newparam3))

(event Input|AxisEvents|InputAxisBrake
  (params (AxisValue :type Float%20%28single-precision%29))
  (Class|WheeledVehicleMovementComponent|SetBrakeInput (Variables|Default|GetVehicleMovement) AxisValue)
  (bind _newparam3 (CallFunction|GetRotationfromAxis (stale Input|AxisEvents|InputAxisMoveRight AxisValue) (stale Input|AxisEvents|InputAxisMoveFoward AxisValue) AxisValue))
  (Class|YawController|UpdateMotionValues (Variables|Default|GetYawController) _newparam3))

(fn ConstructionScript
  (|CallParentFunction))

(fn GetRotationfromAxis
  (params (Turn :type Float%20%28single-precision%29) (Thrust :type Float%20%28single-precision%29) (Brake :type Float%20%28single-precision%29))
  (bind _output_get (Variables|Default|SetCurrentXRotation (Math|Interpolation|FInterpTo (Variables|Default|GetCurrentXRotation) (* (Math|Integer|Clamp(Integer) (Math|Float|Truncate (* (Class|WheeledVehicleMovementComponent|GetForwardSpeed (Variables|Default|GetVehicleMovement)) 0.036)) 0 10) Turn) (Utilities|Time|GetWorldDeltaSeconds) 1.0)))
  (bind _output_get_2 (Variables|Default|SetCurrentYRotation (Math|Interpolation|FInterpTo (Variables|Default|GetCurrentYRotation) (* (Math|Integer|Clamp(Integer) (Math|Float|Truncate (* (Class|WheeledVehicleMovementComponent|GetForwardSpeed (Variables|Default|GetVehicleMovement)) 0.036)) 0 10) (- Thrust Brake)) (Utilities|Time|GetWorldDeltaSeconds) 1.0)))
  (return (Math|Rotator|MakeRotator _output_get _output_get_2 0.0)))