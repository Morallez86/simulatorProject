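; VR-oriented Mercedes vehicle Blueprint that the player drives through axis inputs.
; On BeginPlay it sets the tracking origin to eye level and adds a Cylinder_Text widget to the viewport.
; MoveFoward, MoveRight and Brake axes pass straight to the VehicleMovement component as throttle, steering and brake input.
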(event EventBeginPlay
  (Class|HeadMountedDisplayFunctionLibrary|SetTrackingOrigin "Eye")
  (bind _returnvalue (UserInterface|CreateWidget "/Game/Carla/Blueprints/Vehicles/MercedesCCC_VR/HUD/Cylinder_Text.Cylinder_Text_C"))
  (UserInterface|Viewport|AddtoViewport _returnvalue 0))

(event Collision|EventActorBeginOverlap
  (params (OtherActor :type Actor%20Object%20Reference)))

(event Input|AxisEvents|InputAxisMoveRight
  (params (AxisValue :type Float%20%28single-precision%29))
  (Class|WheeledVehicleMovementComponent|SetSteeringInput (Variables|Default|GetVehicleMovement) AxisValue))

(event Input|AxisEvents|InputAxisMoveFoward
  (params (AxisValue :type Float%20%28single-precision%29))
  (Class|WheeledVehicleMovementComponent|SetThrottleInput (Variables|Default|GetVehicleMovement) AxisValue))

(event Input|AxisEvents|InputAxisBrake
  (params (AxisValue :type Float%20%28single-precision%29))
  (Class|WheeledVehicleMovementComponent|SetBrakeInput (Variables|Default|GetVehicleMovement) AxisValue))

(fn ConstructionScript
  (|CallParentFunction))